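; BP_PreventedTeleportArea is a VR teleport-item actor that, by its name, marks an area where teleporting is prevented.
; Its Construction Script passes four corner components (LT, LB, RT, RB) and their matching socket components to ResetLocationAndScale.
; That helper sets each component to unit world scale and moves it to its socket, so corners keep their size when the area is scaled.
; It contains no active runtime logic.
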(event EventBeginPlay)

(event Collision|EventActorBeginOverlap
  (params (OtherActor :type Actor%20Object%20Reference)))

(event EventTick
  (params (DeltaSeconds :type Float%20%28single-precision%29)))

(fn ConstructionScript
  (CallFunction|ResetLocationandScale (Variables|Default|GetLT) (Variables|Default|GetLT_socket))
  (CallFunction|ResetLocationandScale (Variables|Default|GetLB) (Variables|Default|GetLB_socket))
  (CallFunction|ResetLocationandScale (Variables|Default|GetRT) (Variables|Default|GetRT_socket))
  (CallFunction|ResetLocationandScale (Variables|Default|GetRB) (Variables|Default|GetRB_socket)))

(fn ResetLocationandScale
  (params (BaseComponent :type Scene%20Component%20Object%20Reference) (Socket :type Scene%20Component%20Object%20Reference))
  (Transformation|SetWorldScale3D BaseComponent "1.000000,1.000000,1.000000")
  (Transformation|SetWorldLocation BaseComponent (Transformation|GetWorldLocation Socket) false false))