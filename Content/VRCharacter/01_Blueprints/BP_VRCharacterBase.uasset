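; VR character base Blueprint that handles player movement, teleportation and right-hand grabbing.
; On BeginPlay it adds the VR input mapping context and hands the child-actor teleport spline trace to the Teleportation component.
; Enhanced Input events drive forward movement, begin or end teleporting by input threshold, and update the right-hand pose from grab ratio while triggering grab press and release.
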(event Input|EnhancedActionEvents|EnhancedInputActionIA_VR_Move
  (params (ActionValue :type Float%20%28double-precision%29) (ElapsedSeconds :type Float%20%28double-precision%29) (TriggeredSeconds :type Float%20%28double-precision%29) (InputAction :type Input%20Action%20Object%20Reference :default "/Game/VRCharacter/10_Settings/Input/IA_VR_Move.IA_VR_Move"))
  (:Triggered
    (Class|VRCharacterBase|CharacterMoveForward ActionValue)))

(event Input|EnhancedActionEvents|EnhancedInputActionIA_VR_Grab_Right
  (params (ActionValue :type Float%20%28double-precision%29) (ElapsedSeconds :type Float%20%28double-precision%29) (TriggeredSeconds :type Float%20%28double-precision%29) (InputAction :type Input%20Action%20Object%20Reference :default "/Game/VRCharacter/10_Settings/Input/IA_VR_Grab_Right.IA_VR_Grab_Right"))
  (:Triggered
    (Class|VRCharacterBase|UpdateRightHandPose 0.0 ActionValue false true)
    (if (>= ActionValue 0.8)
      (Class|VRCharacterBase|RightGrabPressed)
      (elif (< ActionValue 0.01)
        (Class|VRCharacterBase|RightGrabReleased :!label _label)
        (Class|VRCharacterBase|UpdateRightHandPose 0.0 0.0 false true))))
  (:Canceled
    (goto _label))
  (:Completed
    (goto _label)))

(event Input|EnhancedActionEvents|EnhancedInputActionIA_VR_Teleport
  (params (ActionValue :type Float%20%28double-precision%29) (ElapsedSeconds :type Float%20%28double-precision%29) (TriggeredSeconds :type Float%20%28double-precision%29) (InputAction :type Input%20Action%20Object%20Reference :default "/Game/VRCharacter/10_Settings/Input/IA_VR_Teleport.IA_VR_Teleport"))
  (bind _teleportation (Variables|Default|GetTeleportation))
  (:Triggered
    (if (>= ActionValue 0.1)
      (Class|Teleportation|BeginTeleport _teleportation ActionValue)
      (else
        (Class|Teleportation|EndTeleport _teleportation :!label _label))))
  (:Completed
    (goto _label)))

(event EventBeginPlay
  ;[1 1 1] Add Mapping Context
  (bind _asplayer_controller (Utilities|Casting|CastToPlayerController (Pawn|GetController)))
  (Input|AddMappingContext (PlayerController|LocalPlayerSubsystems|GetEnhancedInputLocalPlayerSubsystem _asplayer_controller) "/Game/VRCharacter/10_Settings/Input/IMC_VR_Inputs.IMC_VR_Inputs" 0 "(bIgnoreAllPressedKeysUntilRelease=True,bForceImmediately=False)")
  ;[1 0.454 0] Set Teleport Trace
  (bind _asteleportation_trace (Utilities|Casting|CastToTeleportationTrace (Variables|/Script/Engine.ChildActorComponent|GetChildActor (Variables|Default|GetBP_Teleport_Spline))))
  (Variables|/Script/VRCharacter.Teleportation|SetTeleportTrace (Variables|Default|GetTeleportation) _asteleportation_trace))

(event Collision|EventActorBeginOverlap
  (params (OtherActor :type Actor%20Object%20Reference)))

(event EventTick
  (params (DeltaSeconds :type Float%20%28single-precision%29)))

(fn ConstructionScript)