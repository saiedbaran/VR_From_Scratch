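; Right VR hand Blueprint with a segmented mesh, debug display and finger-tap toggle for grabbity grabbing.
; Construction attaches each Detail piece to the HandMesh socket derived from its name; BeginPlay gives the pieces one shared dynamic material.
; A left-index overlap on DebugAreaCollider calls ToggleGrabbityGrabbing, with a cooldown.
; Debug components start hidden; events update their text widget or toggle visibility after a hologram burst.
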(event OnComponentBeginOverlap(DebugAreaCollider)
  (params (OverlappedComponent :type Primitive%20Component%20Object%20Reference) (OtherActor :type Actor%20Object%20Reference) (OtherComp :type Primitive%20Component%20Object%20Reference) (OtherBodyIndex :type Integer) (bFromSweep :type Boolean) (SweepResult :type Hit%20Result%20Structure%20%28by%20ref%29))
  ;[0 0.4339 1] Switch Interaction Mode
  (if (Utilities|Array|ContainsItem (Variables|/Script/Engine.ActorComponent|GetComponentTags OtherComp) "tag_Index_left")
    (if (> (Utilities|Time|GetTimeSeconds) (+ (Variables|Default|GetLastDebugToggleTime) (Variables|Default|GetDelayBetweenToggleDebug)))
      (Variables|Default|SetLastDebugToggleTime (Utilities|Time|GetTimeSeconds))
      (Class|HandSkeletalActor|ToggleGrabbityGrabbing))))

(event EventBeginPlay
  (CallFunction|CreateDynamicMaterialIntance)
  (CallFunction|InitializeDebugComponents))

(event Collision|EventActorBeginOverlap
  (params (OtherActor :type Actor%20Object%20Reference)))

(event EventTick
  (params (DeltaSeconds :type Float%20%28single-precision%29)))

(event EventUpdateDebugText
  (params (VariableName :type String) (VariableValue :type String))
  (bind _debug_text_widget (Variables|Default|GetDebug%20Text%20Widget))
  ;[1 1 1] Debug Visualization
  (if (Variables|Default|GetbDebugVisualizationEnabled)
    (Variables|/Game/VRCharacter/05_UI/Debug/WBP_DebugText.WBP_DebugText_C|SetVariableName _debug_text_widget (Utilities|Text|ToText(String) VariableName))
    (Variables|/Game/VRCharacter/05_UI/Debug/WBP_DebugText.WBP_DebugText_C|SetValueText _debug_text_widget (Utilities|Text|ToText(String) VariableValue))
    (Default|UpdateValueFontSize _debug_text_widget)))

(event EventToggleDebugVisualization
  (bind _debugcomponents (Variables|Default|GetDebugComponents))
  ;[1 1 1] Debug Visualization
  (Niagara|SpawnSystemAttached "/Game/VRCharacter/04_FX/LaserHologram/NS_Hologram_FirstBurst.NS_Hologram_FirstBurst" (Variables|Default|GetHandMesh) "None" (Transformation|GetWorldLocation (Variables|Default|GetNS_LaserHologram)) "0, 0, 0" "KeepWorldPosition" true)
  (Utilities|FlowControl|Delay 0.5)
  (Development|SetHiddeninGame _debugcomponents (not (Variables|/Script/Engine.SceneComponent|GetbHiddenInGame _debugcomponents)) true)
  (Variables|Default|SetbDebugVisualizationEnabled (not (Variables|Default|GetbDebugVisualizationEnabled))))

(fn ConstructionScript
  (CallFunction|AttachtoHand))

(fn AttachtoHand
  (bind _arrayelement (Utilities|Array|ReverseforEachLoop (Components|GetChildrenComponents (Variables|Default|GetDetail) false))
    (:LoopBody
      (Transformation|AttachComponentToComponent _arrayelement (Variables|Default|GetHandMesh) (Utilities|String|StringToName (Utilities|String|Replace (Utilities|String|Replace (Utilities|GetObjectName _arrayelement) "Hand_Nanite_SM_") "_GRP")) "KeepWorld" "KeepWorld" "KeepWorld" true))))

(fn InitializeDebugComponents
  (bind _widget (Variables|Default|GetWidget))
  (Variables|Default|SetDebugWidgetComponent _widget)
  (bind _aswbp_debug_text (Utilities|Casting|CastToWBP_DebugText (UserInterface|GetWidget _widget)))
  (Variables|Default|SetDebug%20Text%20Widget _aswbp_debug_text)
  (Development|SetHiddeninGame (Variables|Default|GetDebugComponents) true true))

(fn CreateDynamicMaterialIntance
  (bind _hand_nanite_sm_middle_02_r_grp (Variables|Default|GetHand_Nanite_SM_middle_02_r_GRP))
  (bind _returnvalue (Rendering|Material|CreateDynamicMaterialInstance _hand_nanite_sm_middle_02_r_grp 0 (Rendering|Material|GetMaterial _hand_nanite_sm_middle_02_r_grp 0) "None" :!class /Script/Engine.PrimitiveComponent))
  (Variables|Default|SetDynamicMaterialInstance _returnvalue)
  (bind _arrayelement (Utilities|Array|ReverseforEachLoop (Components|GetChildrenComponents (Variables|Default|GetHandMesh) false))
    (:LoopBody
      (bind _asstatic_mesh_component (Utilities|Casting|CastToStaticMeshComponent _arrayelement))
      (Rendering|Material|SetMaterial _asstatic_mesh_component 0 (Variables|Default|GetDynamicMaterialInstance)))))